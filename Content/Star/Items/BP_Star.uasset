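; BP_Star is a collectible star that bobs on a sine wave and spins every tick.
; Overlapping Box1 the first time marks its StarIndex in the GameState's CollectedStars array and increments StarTotal.
; BeginPlay reads that array and shares the visual update, turning collected stars to glass with a blue light instead of removing them.
; The spin is a fixed step per frame, so its speed depends on frame rate.
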(event OnComponentBeginOverlap(Box1)
  (params (OtherActor :type Actor%20Object%20Reference) (OtherComp :type Primitive%20Component%20Object%20Reference) (OtherBodyIndex :type Integer) (bFromSweep :type Boolean) (SweepResult :type Hit%20Result%20Structure%20%28by%20ref%29))
  ;[1 1 1] Touch Star
  (if (not (Variables|Default|GetisCollected)) ; Star Already collected?
    (Variables|Default|SetisCollected true)
    (Utilities|Casting|CastTo (Game|GetGameState))
    (Utilities|Array|SetArrayElem (Variables|Default|GetCollectedStars) (Variables|Default|GetStarIndex) (Variables|Default|GetisCollected))
    (Variables|Default|SetStarTotal (+ (Variables|Default|GetStarTotal) 1))
    ;[1 1 1] Change to glass if its collected
    (if (Variables|Default|GetisCollected)
      (Rendering|Material|SetMaterial (Variables|Default|GetStarMesh) 0 "/Game/Star/Items/Meshes/Materials/StarGlass_MAT.StarGlass_MAT")
      (Rendering|Components|Light|SetLightColor (Variables|Default|GetPointLight1) "(R=0.120871,G=0.224963,B=0.710000,A=1.000000)"))))

(event EventBeginPlay
  ;[1 1 1] Check if star has collected when the game starts
  (Utilities|Casting|CastTo (Game|GetGameState))
  (Variables|Default|SetisCollected (Utilities|Array|Get(acopy) (Variables|Default|GetCollectedStars) (Variables|Default|GetStarIndex)))
  ;[1 1 1] Change to glass if its collected
  (if (Variables|Default|GetisCollected)
    (Rendering|Material|SetMaterial (Variables|Default|GetStarMesh) 0 "/Game/Star/Items/Meshes/Materials/StarGlass_MAT.StarGlass_MAT")
    (Rendering|Components|Light|SetLightColor (Variables|Default|GetPointLight1) "(R=0.120871,G=0.224963,B=0.710000,A=1.000000)")))

(event EventTick
  (params (DeltaSeconds :type Float%20%28single-precision%29))
  (Utilities|FlowControl|Sequence
    (:then_0
      ;[1 1 1] Bounce the star
      (Transformation|SetRelativeLocation (Variables|Default|GetStarMesh) (Math|Vector|MakeVector 0.0 0.0 (* (Math|Trig|Sin(Radians) (* (Utilities|Time|GetGameTimeinSeconds) 1.0)) 32.0)) false))
    (:then_1
      ;[1 1 1] Spin the Star
      (Transformation|AddRelativeRotation (Variables|Default|GetStarMesh) "0,4.000000,0.000000" false))))

(fn ConstructionScript)