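; BP_Scrap is a collectible scrap item that adds to the player's Scrap total.
; On CollectItem, it casts player character 0 to StarPlayer, adds ScrapValue to its Scrap, then destroys itself.
; Its construction script runs the parent's script, then picks a random static mesh from ScrapMeshes to vary its appearance.
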(event EventCollectItem
  (bind _asstar_player (Utilities|Casting|CastToStarPlayer (Game|GetPlayerCharacter 0)))
  (bind _output_get (Variables|/Game/Star/Player/StarPlayer.StarPlayer_C|SetScrap _asstar_player (+ (stale _output_get) (Variables|Default|GetScrapValue))))
  (Actor|DestroyActor))

(fn ConstructionScript
  (bind _scrapmeshes (Variables|Default|GetScrapMeshes))
  (|CallParentFunction)
  (Components|StaticMesh|SetStaticMesh (Utilities|Array|Get(acopy) _scrapmeshes (Math|Random|RandomIntegerinRange 0 (Utilities|Array|LastIndex _scrapmeshes)))))