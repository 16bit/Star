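; Health pickup actor that grants healing to the player character once collected, then removes itself from the world.
; It calls the parent Tick, noted as driving rotation and bobbing, then polls the inherited IsCollected flag every frame.
; When the flag is set, it casts player character 0, adds a fixed amount to its HealHealth variable and destroys the pickup.
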(event EventTick
  (params (DeltaSeconds :type Float%20%28single-precision%29))
  ;[1 1 1] Get Ticks for rotating and bobbing
  (|CallParentFunction DeltaSeconds)
  ;[1 1 1] See if this pickup has been collected by looking at parent variable
  (bind _asbp_pick_up_parent (Utilities|Casting|CastTo self))
  (if (Variables|Default|GetbIsCollected _asbp_pick_up_parent)
    (bind _asmy_character (Utilities|Casting|CastTo (Game|GetPlayerCharacter 0)))
    (bind _output_get (Variables|Default|SetHeal%20Health _asmy_character (+ (stale _output_get) 5)))
    (Actor|DestroyActor)))

(fn ConstructionScript
  (|CallParentFunction))