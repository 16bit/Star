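; StarGameState holds collected stars, star total and total game time, and persists them through a StarSaveSlot save object in "Slot1".
; BeginPlay copies saved values into the game state, or writes a fresh save when none exists.
; SaveGame reloads the slot and copies current values into it, but its final SaveGameToSlot call shows no save object connected.
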(event Custom|SaveGame
  (bind _returnvalue (SaveGame|LoadGamefromSlot "Slot1"))
  (bind _asstar_save_slot (Utilities|Casting|CastToStarSaveSlot _returnvalue))
  (Variables|Default|SetStarSaveSlot _asstar_save_slot)
  (Utilities|FlowControl|Sequence
    (:then_0
      (Variables|/Game/Star/Blueprints/StarSaveSlot.StarSaveSlot_C|SetSAVECollectedStars (Variables|Default|GetStarSaveSlot) (Variables|Default|GetCollectedStars)))
    (:then_1
      (Variables|/Game/Star/Blueprints/StarSaveSlot.StarSaveSlot_C|SetSAVEStarTotal (Variables|Default|GetStarSaveSlot) (Variables|Default|GetStarTotal)))
    (:then_2
      (Variables|/Game/Star/Blueprints/StarSaveSlot.StarSaveSlot_C|SetSAVETotalGameTime (Variables|Default|GetStarSaveSlot) (Variables|Default|GetTotalGameTime)))
    (:then_3
      (SaveGame|SaveGametoSlot 0 "Slot1"))))

(event EventBeginPlay
  (bind _returnvalue (SaveGame|DoesSaveGameExist "Slot1"))
  (if _returnvalue
    ;[1 1 1] Load the variables from the save slot and put them into the gamestates variables
    (bind _returnvalue_2 (SaveGame|LoadGamefromSlot "Slot1"))
    (bind _asstar_save_slot (Utilities|Casting|CastToStarSaveSlot _returnvalue_2))
    (Variables|Default|SetStarSaveSlot _asstar_save_slot)
    (Utilities|FlowControl|Sequence
      (:then_0
        (Variables|Default|SetCollectedStars (Variables|/Game/Star/Blueprints/StarSaveSlot.StarSaveSlot_C|GetSAVECollectedStars (Variables|Default|GetStarSaveSlot))))
      (:then_1
        (Variables|Default|SetStarTotal (Variables|/Game/Star/Blueprints/StarSaveSlot.StarSaveSlot_C|GetSAVEStarTotal (Variables|Default|GetStarSaveSlot))))
      (:then_2
        (Variables|Default|SetTotalGameTime (Variables|/Game/Star/Blueprints/StarSaveSlot.StarSaveSlot_C|GetSAVETotalGameTime (Variables|Default|GetStarSaveSlot)))))
    (else
      ;[1 1 1] If there is no save slot create one
      (bind _returnvalue_3 (SaveGame|CreateSaveGameObject "/Game/Star/Blueprints/StarSaveSlot.StarSaveSlot_C"))
      (bind _asstar_save_slot_2 (Utilities|Casting|CastToStarSaveSlot _returnvalue_3))
      (SaveGame|SaveGametoSlot _asstar_save_slot_2 "Slot1"))))

(fn ConstructionScript)