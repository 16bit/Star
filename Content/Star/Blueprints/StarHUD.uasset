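; StarHUD is a HUD with a pause menu, toggled through ToggleMenu, plus click and release handling for Resume and Save hit boxes.
; Resume closes the menu and unpauses, Save calls the game mode, and a left click also clears MenuOpen.
; DrawButton centers texture, text and hit box on a point.
; The code drawing the menu or cursor, star total and time is disconnected from DrawHUD, so it never runs.
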(event Custom|Event%20Toggle%20Menu
  (params (Menu%20Open :type Boolean))
  (Variables|Default|SetMenu%20Open Menu%20Open))

(event EventHitBoxClick
  (params (BoxName :type Name :default "None"))
  (switch name BoxName
    (:Resume
      (Variables|Default|SetResumePressed true))
    (:Save
      (Variables|Default|SetSave%20Pressed true))
    (:Quit
      (Variables|Default|SetQuit%20Pressed true))))

(event EventHitBoxRelease
  (params (BoxName :type Name :default "None"))
  (bind _returnvalue (Game|GetPlayerController 0))
  (switch name BoxName
    (:Resume
      (if (Variables|Default|GetResumePressed)
        (Variables|Default|SetMenu%20Open false)
        (Variables|/Script/Engine.PlayerController|SetbShowMouseCursor _returnvalue false)
        (Variables|/Script/Engine.PlayerController|SetbEnableClickEvents _returnvalue false)
        (Game|SetGamePaused false)))
    (:Save
      (if (Variables|Default|GetSave%20Pressed)
        (Utilities|Casting|CastTo (Game|GetGameMode))
        (CallFunction|Save)
        (Variables|Default|SetSave%20Pressed false)))))

(event EventDrawHUD
  (params (SizeX :type Integer) (SizeY :type Integer)))

(event Input|MouseEvents|LeftMouseButton
  (:Pressed
    (Variables|Default|SetMenu%20Open false)))

(fn ConstructionScript)

(fn DrawButton
  (params (Button%20Screen%20Location :type Vector%202D%20Structure) (Button%20Text :type String) (Hitbox%20Name :type Name) (Button%20Texture :type Texture%202D%20Object%20Reference) (Text%20Color :type Linear%20Color%20Structure) (Scale :type Float%20%28single-precision%29))
  (bind _returnvalue (Math|Vector2D|MakeVector2D 128.0 64.0))
  (bind (_outwidth _outheight) (Class|HUD|GetTextSize Button%20Text 0 1.0))
  (bind _returnvalue_2 (Math|Vector2D|MakeVector2D _outwidth _outheight))
  (bind _returnvalue_3 (* _returnvalue Scale))
  (bind _returnvalue_4 (- Button%20Screen%20Location _returnvalue_3))
  (bind _returnvalue_5 (/ _returnvalue_2 2.0))
  (bind _returnvalue_6 (* _returnvalue_5 Scale))
  (bind (_x _y) (Math|Vector2D|BreakVector2D _returnvalue_4))
  (bind _returnvalue_7 (- Button%20Screen%20Location _returnvalue_6))
  (bind (_x_2 _y_2) (Math|Vector2D|BreakVector2D _returnvalue_7))
  (Class|HUD|DrawTextureSimple Button%20Texture _x _y Scale false) ; Draw button texture
  (HUD|DrawText Button%20Text Text%20Color _x_2 _y_2 0 Scale false) ; Draw button text
  (Class|HUD|AddHitBox _returnvalue_4 (* (Math|Vector2D|MakeVector2D 256.0 128.0) Scale) Hitbox%20Name false) ; Add a hit box for the button
)