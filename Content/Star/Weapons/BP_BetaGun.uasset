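; BP_BetaGun is a modular gun Blueprint assembled at runtime from a body class and a barrel class.
; On BeginPlay, UpdateParts destroys existing parts, spawns the body on the root and snaps the barrel to the body's barrel socket.
; It then sums base values and both parts' bonuses into the gun's stats.
; Fire passes the barrel mesh's Fire socket transform to the parent implementation.
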(event Custom|Update%20Parts
  (bind _returnvalue (Transformation|GetActorTransform))
  (Actor|DestroyActor (Variables|Default|GetBarrelActor))
  (Utilities|FlowControl|Sequence
    (:then_0
      ;[1 1 1] Spawn Body and Attach to root
      (bind _returnvalue_2 (Game|SpawnActorfromClass (Variables|Default|GetBodyClass) _returnvalue false 0))
      (Class|Actor|AttachRootComponentto _returnvalue_2 (Variables|Default|GetDefaultSceneRoot) "None" "SnapToTarget" true)
      (bind _asgun_parts (Utilities|Casting|CastToGunParts _returnvalue_2))
      (Variables|Default|SetBodyActor _asgun_parts))
    (:then_1
      ;[1 1 1] Spawn Barrel and Attach to Body
      (bind _returnvalue_3 (Game|SpawnActorfromClass (Variables|Default|GetBarrelClass) _returnvalue false 0))
      (Class|Actor|AttachRootComponenttoActor _returnvalue_3 _returnvalue_2 "Socket_Barrel" "SnapToTarget" true)
      (bind _asbeta_gun_barrel (Utilities|Casting|CastToBetaGunBarrel _returnvalue_3))
      (bind _output_get (Variables|Default|SetBarrelActor _asbeta_gun_barrel)))
    (:then_2
      ;[1 1 1] Update Stats for pieces selected
      (Utilities|FlowControl|Sequence
        (:then_0
          (Variables|Default|SetPower (+ (Variables|/Game/Star/Weapons/Parts/GunParts.GunParts_C|GetPower (Variables|Default|GetBodyActor)) 1e+01 (Variables|/Game/Star/Weapons/Parts/GunParts.GunParts_C|GetPower (Variables|Default|GetBarrelActor)))))
        (:then_1
          (Variables|Default|SetEnergy (+ (Variables|/Game/Star/Weapons/Parts/GunParts.GunParts_C|GetEnergy (Variables|Default|GetBodyActor)) 1e+02 (Variables|/Game/Star/Weapons/Parts/GunParts.GunParts_C|GetEnergy (Variables|Default|GetBarrelActor)))))
        (:then_2
          (Variables|Default|SetAccuracy (+ (Variables|/Game/Star/Weapons/Parts/GunParts.GunParts_C|GetAccuracy (Variables|Default|GetBodyActor)) 75.0 (Variables|/Game/Star/Weapons/Parts/GunParts.GunParts_C|GetAccuracy (Variables|Default|GetBarrelActor)))))
        (:then_3
          (Variables|Default|SetSpeed (+ (Variables|/Game/Star/Weapons/Parts/GunParts.GunParts_C|GetSpeed (Variables|Default|GetBodyActor)) 1e+03 (Variables|/Game/Star/Weapons/Parts/GunParts.GunParts_C|GetSpeed (Variables|Default|GetBarrelActor)))))
        (:then_4
          (Variables|Default|SetFireRate (+ (Variables|/Game/Star/Weapons/Parts/GunParts.GunParts_C|GetFireRate (Variables|Default|GetBodyActor)) 1.0 (Variables|/Game/Star/Weapons/Parts/GunParts.GunParts_C|GetFireRate (Variables|Default|GetBarrelActor)))))))))

(event EventBeginPlay
  (CallFunction|UpdateParts))

(event EventActorBeginOverlap
  (params (OtherActor :type Actor%20Object%20Reference)))

(event EventTick
  (params (DeltaSeconds :type Float%20%28single-precision%29)))

(event EventFire
  (params (Spawn%20Transform :type Transform))
  (|CallParentFunction (Transformation|GetSocketTransform (Variables|/Game/Star/Weapons/Parts/GunParts.GunParts_C|GetStaticMesh (stale Custom|Update%20Parts _output_get)) "Fire" "RTS_World")))

(fn ConstructionScript)